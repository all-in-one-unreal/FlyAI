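; PathVolume is a box volume that samples its space on a 3D grid and visualizes it with debug box traces.
; The construction script sizes the box from BoxExtent, and a looping timer started on BeginPlay repeatedly calls DrawPositions.
; That function splits the volume by DivideBy and runs a Visibility box trace at interior grid points, drawn for one frame.
; Trace results are unused, and Sphere1 rotates slightly after each trace.
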(event EventBeginPlay
  (Utilities|Time|SetTimerbyFunctionName 0 "DrawPositions" 0.05 true))

(fn ConstructionScript
  (Components|Box|SetBoxExtent (Variables|Default|GetVolume) (Variables|Default|GetBoxExtent) true))

(fn DrawPositions
  (bind _divideby (Variables|Default|GetDivideBy))
  (bind _volume (Variables|Default|GetVolume))
  (bind _returnvalue (Components|Box|GetScaledBoxExtent _volume))
  (bind _returnvalue_2 (* _returnvalue 2.0))
  (bind _returnvalue_3 (/ _returnvalue_2 _divideby))
  (bind _returnvalue_4 (/ _returnvalue_2 _returnvalue_3))
  (bind (_x _y _z) (Math|Vector|BreakVector _returnvalue_4))
  (for _index (range 1 (- (Math|Float|Floor _x) 1))
    (LocalVariables|SetX _index)
    (for _index_2 (range 1 (- (Math|Float|Floor _y) 1))
      (LocalVariables|SetY _index_2)
      (for _index_3 (range 1 (- (Math|Float|Floor _z) 1))
        (LocalVariables|SetZ _index_3)
        (Collision|BoxTraceByChannel (+ (- (Transformation|GetActorLocation) _returnvalue) (* _returnvalue_3 (Math|Vector|MakeVector (Math|Conversions|ToFloat(Integer) (LocalVariables|GetX)) (Math|Conversions|ToFloat(Integer) (LocalVariables|GetY)) (Math|Conversions|ToFloat(Integer) (LocalVariables|GetZ))))) (+ (+ (- (Transformation|GetActorLocation) _returnvalue) (* _returnvalue_3 (Math|Vector|MakeVector (Math|Conversions|ToFloat(Integer) (LocalVariables|GetX)) (Math|Conversions|ToFloat(Integer) (LocalVariables|GetY)) (Math|Conversions|ToFloat(Integer) (LocalVariables|GetZ))))) "0.001000,0.001000,0.001000") _returnvalue_3 (Transformation|GetActorRotation) "TraceTypeQuery1" false 0 "ForOneFrame" false)
        (Transformation|AddLocalRotation (Variables|Default|GetSphere1) "0,1.500000, 0" false)))))